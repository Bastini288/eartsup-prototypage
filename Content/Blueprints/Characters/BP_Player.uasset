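; Player character Blueprint that implements a melee attack on the IA_Attaque input.
; The input plays the AM_Attaque montage behind an OnAttaque guard and starts a looping timer, cleared when the montage completes.
; The Attaque event sphere-overlaps Pawns at HitLocation, excluding self, and sends each a PrendreDegat damage message.
; It keeps no hit list, so repeated calls can damage the same target again.
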(event Custom|Attaque
  (bind _outactors (Collision|SphereOverlapActors (Transformation|GetWorldLocation (Variables|Default|GetHitLocation)) 1e+02 (Utilities|Array|MakeArray "ObjectTypeQuery3") 0 (Utilities|Array|MakeArray self)))
  (for _array_element _outactors
    (Class|Degat|PrendreDegat(Message) _array_element (Variables|Default|GetAttaqueDamage))))

(event Input|EnhancedActionEvents|EnhancedInputActionIA_Attaque
  (params (ActionValue :type Boolean) (ElapsedSeconds :type Float%20%28double-precision%29) (TriggeredSeconds :type Float%20%28double-precision%29) (InputAction :type Input%20Action%20Object%20Reference :default "/Game/Inputs/IA_Attaque.IA_Attaque"))
  (Variables|Default|GetOnAttaque
    (:then)
    (:else
      (Variables|Default|SetOnAttaque true)
      (Animation|Montage|PlayMontage (Variables|Character|GetMesh) "/Game/Animation/AM_Attaque.AM_Attaque"
        (:then
          (bind _returnvalue (Utilities|Time|SetTimerbyEvent (EventDispatchers|CreateEvent :!event Custom|Attaque) 0.1 true))
          (Variables|Default|SetTimerAttaque _returnvalue))
        (:OnCompleted
          (Variables|Default|SetOnAttaque false)
          (Utilities|Time|ClearandInvalidateTimerbyHandle (Variables|Default|GetTimerAttaque)))))))

(fn ConstructionScript)