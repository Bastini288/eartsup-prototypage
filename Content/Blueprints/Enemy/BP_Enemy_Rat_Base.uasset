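; Base rat enemy Blueprint that handles taking damage and dying.
; PrendreDegat (take damage) uses a CanHit flag and a one-second timer as a hit cooldown, then applies damage through ReceiveDomage and prints current HP as debug output.
; A surviving hit spawns a Niagara blood effect, while a lethal one calls Die, which spawns an explosion effect and destroys the actor.
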(event Custom|ReleaseCanHit
  (Variables|Default|SetCanHit true))

(event Custom|Die
  (bind _returnvalue (Transformation|GetActorLocation))
  (Niagara|SpawnSystematLocation "/Game/VFX/Explosion/NS_Super_Explosion.NS_Super_Explosion" (Math|Vector|MakeVector (.x _returnvalue) (.y _returnvalue) (+ (.z _returnvalue) 2e+01)))
  (Actor|DestroyActor))

(event EventBeginPlay)

(event Collision|EventActorBeginOverlap
  (params (OtherActor :type Actor%20Object%20Reference)))

(event EventTick
  (params (DeltaSeconds :type Float%20%28single-precision%29)))

(event EventPrendreDegat
  (params (degat :type Integer))
  (bind _returnvalue (Transformation|GetActorLocation))
  (Variables|Default|GetCanHit
    (:then
      (Variables|Default|SetCanHit false)
      (Utilities|Time|SetTimerbyEvent (EventDispatchers|CreateEvent :!event Custom|ReleaseCanHit) 1.0)
      (bind _returnvalue_2 (Class|BaseCharacter|ReceiveDomage degat))
      (Development|PrintString (Utilities|String|ToString(Integer) (Variables|Default|GetCurrentHP)) true true "(R=0.000000,G=0.660000,B=1.000000,A=1.000000)" 1.0 "aaa")
      (if _returnvalue_2
        (CallFunction|Die)
        (else
          (Niagara|SpawnSystematLocation "/Game/VFX/NS_Blood.NS_Blood" (Math|Vector|MakeVector (.x _returnvalue) (.y _returnvalue) (+ (.z _returnvalue) 2e+01))))))
    (:else)))

(fn ConstructionScript)